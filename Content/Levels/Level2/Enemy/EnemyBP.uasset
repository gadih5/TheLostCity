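; Spear-wielding melee enemy character for Level 2 that chases the player and counts toward the level win.
; It repeatedly re-issues AIMoveTo at a randomized walk speed, looping a stationary spear montage while the player overlaps its attack range.
; Spear collision deals damage, gated by CanHit, which is never re-armed in this graph.
; Damage causes a stagger or death with random montages; the tenth player kill opens WinLevel.
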(event `self.ReceiveBeginPlay`
  ;[1 1 1] Init speed
  (bind _asue_4asp_character (cast `/Game/Levels/Level2/Character/Ue4ASP_Character` (`GameplayStatics.GetPlayerCharacter` 0)))
  (bind _output_get (set `self.Char REF` _asue_4asp_character))
  (`self.Chase Player` _output_get)
  (set `CharacterMovementComponent.MaxWalkSpeed` (select `int` (`KismetMathLibrary.RandomInteger` 2) :`0` 200.0 :`1` 250.0 :`2` 300.0 :!type "Float (single-precision)") (`self.CharacterMovement`)))

(event `Chase Player`
  (params (`Player To Chase` :type "/Game/Levels/Level2/Character/Ue4ASP_Character Object Reference"))
  ;[1 1 1] Chasing
  (if (not (`self.IsDead?`))
    (`|AIMoveTo` self (0.0 0.0 0.0) `Player To Chase`
      (:`OnSuccess`
        (`self.Chase Player` (`self.Char REF`)))
      (:`OnFail`
        (`self.Chase Player` (`self.Char REF`))))))

(event `self.ReceiveAnyDamage`
  (params (Damage :type "Float (single-precision)") (DamageType :type "DamageType Object Reference") (InstigatedBy :type "Controller Object Reference") (DamageCauser :type "Actor Object Reference"))
  (bind _returnvalue (`self.K2_GetActorLocation`))
  ;[1 1 1] Damaging
  (if (not (`self.IsDead?`))
    (bind _output_get (set `self.Health` (`KismetMathLibrary.FClamp` (- (`self.Health`) Damage) 0.0 100.0)))
    (if (== _output_get 0.0)
      (`GameplayStatics.PlaySoundAtLocation` "/Game/Sound/DeathCue.DeathCue" _returnvalue (struct) 1.0 1.0 0.0 null null null)
      (`CharacterMovementComponent.DisableMovement` (`self.CharacterMovement`))
      (set `self.IsDead?` true)
      (`self.PlayAnimMontage` (select `int` (`KismetMathLibrary.RandomInteger` 3) :`0` "/Game/Levels/Level2/Enemy/animations/Death_1_Montage.Death_1_Montage" :`1` "/Game/Levels/Level2/Enemy/animations/Death_2_Montage.Death_2_Montage" :`2` "/Game/Levels/Level2/Enemy/animations/Death_3_Montage.Death_3_Montage" :`3` "/Game/Levels/Level2/Enemy/animations/Death_4_Montage.Death_4_Montage" :!type "AnimMontage Object Reference"))
      (`PrimitiveComponent.SetCollisionEnabled` (`self.CapsuleComponent`) "NoCollision")
      (`|ExecutionSequence`
        (:`then_0`
          (bind _asue_4asp_character (cast `/Game/Levels/Level2/Character/Ue4ASP_Character` (`GameplayStatics.GetPlayerCharacter` 0)))
          (bind _result (`/Engine/EditorBlueprintResources/StandardMacros.IncrementInt` (`/Game/Levels/Level2/Character/Ue4ASP_Character.Kills` _asue_4asp_character))
            (:`  `
              (if (== _result 10)
                (`GameplayStatics.SetGamePaused` false)
                (`KismetSystemLibrary.Delay` 3.0)
                (`GameplayStatics.OpenLevel` "WinLevel")))))
        (:`then_1`
          (`KismetSystemLibrary.Delay` 60.0)
          (`self.K2_DestroyActor`)))
      (else
        (`GameplayStatics.PlaySoundAtLocation` "/Game/Sound/DamageCue.DamageCue" _returnvalue (struct) 1.0 1.0 0.0 null null null)
        (`CharacterMovementComponent.DisableMovement` (`self.CharacterMovement`))
        (`GameplayStatics.SpawnEmitterAtLocation` "/Game/Realistic_Starter_VFX_Pack_Vol2/Particles/Blood/P_Blood_Splat_Cone.P_Blood_Splat_Cone" (`SceneComponent.GetSocketLocation` (`self.Mesh`) "None") (struct) (1.5 1.5 1.5))
        (bind _returnvalue_2 (`self.PlayAnimMontage` (select `int` (`KismetMathLibrary.RandomInteger` 3) :`0` "/Game/Levels/Level2/Enemy/animations/Hit_1_Montage.Hit_1_Montage" :`1` "/Game/Levels/Level2/Enemy/animations/Hit_2_Montage.Hit_2_Montage" :`2` "/Game/Levels/Level2/Enemy/animations/Hit_3_Montage.Hit_3_Montage" :`3` "/Game/Levels/Level2/Enemy/animations/Hit_4_Montage.Hit_4_Montage" :!type "AnimMontage Object Reference")))
        (`KismetSystemLibrary.Delay` _returnvalue_2)
        (if (not (`self.IsDead?`))
          (`CharacterMovementComponent.SetMovementMode` (`self.CharacterMovement`) "MOVE_Walking" 0))))))

(event `self.Attack_Range.OnComponentBeginOverlap`
  (params (OverlappedComponent :type "PrimitiveComponent Object Reference") (OtherActor :type "Actor Object Reference") (OtherComp :type "PrimitiveComponent Object Reference") (OtherBodyIndex :type Integer) (bFromSweep :type Boolean) (SweepResult :type "HitResult Structure (by ref)"))
  ;[1 1 1] Attack Range
  (if (and (== OtherActor (`self.Char REF`)) (not (`self.isAttacking?`)) (not (`self.IsDead?`)))
    (set `self.can attack?` true)
    (set `self.isAttacking?` true :!label _label)
    (`|ExecutionSequence`
      (:`then_0`
        (`|PlayMontage` (`self.Mesh`) "/Game/AnimStarterPack/spear_attack_mont.spear_attack_mont"
          (:`OnCompleted`
            (set `self.isAttacking?` false)
            (`|ExecutionSequence`
              (:`then_0`
                (if (`self.can attack?`)
                  (goto _label)))
              (:`then_1`
                (`CharacterMovementComponent.SetMovementMode` (`self.CharacterMovement`) "MOVE_Walking" 0))))))
      (:`then_1`
        (`CharacterMovementComponent.DisableMovement` (`self.CharacterMovement`))))))

(event `self.Attack_Range.OnComponentEndOverlap`
  (params (OverlappedComponent :type "PrimitiveComponent Object Reference") (OtherActor :type "Actor Object Reference") (OtherComp :type "PrimitiveComponent Object Reference") (OtherBodyIndex :type Integer))
  ;[1 1 1] End Attack
  (if (and (== OtherActor (`self.Char REF`)) (`self.can attack?`) (not (`self.IsDead?`)))
    (set `self.can attack?` false)))

(event `self.spear_collision.OnComponentBeginOverlap`
  (params (OverlappedComponent :type "PrimitiveComponent Object Reference") (OtherActor :type "Actor Object Reference") (OtherComp :type "PrimitiveComponent Object Reference") (OtherBodyIndex :type Integer) (bFromSweep :type Boolean) (SweepResult :type "HitResult Structure (by ref)"))
  ;[1 1 1] Attack (hit)
  (if (and (== OtherActor (`self.Char REF`)) (`self.can hit?`) (not (`/Game/Levels/Level2/Character/Ue4ASP_Character.IsDead?` (`self.Char REF`))))
    (set `self.can hit?` false)
    (`/Game/Levels/Level2/Character/Ue4ASP_Character.Take Damage` (`self.Char REF`) (`KismetMathLibrary.SelectFloat` 9.0 6.0 (`KismetMathLibrary.RandomBool`)))))

(fn `UserConstructionScript`)